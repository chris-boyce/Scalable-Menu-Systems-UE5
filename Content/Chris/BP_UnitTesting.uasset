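; BP_UnitTesting is a test actor that runs unit tests for data structures when play begins.
; BeginPlay finds the BP_ScoreboardManager in the level, stores it as LocalSBM, then calls each test function in sequence.
; The test names cover binary tree insertion, search and traversal, linked list editing and position lookup, and stack operations; their bodies are not included here.
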(event `self.ReceiveBeginPlay`
  (bind _returnvalue (`GameplayStatics.GetActorOfClass` "/Game/Chris/BP_ScoreboardManager.BP_ScoreboardManager_C"))
  (set `self.LocalSBM` _returnvalue)
  (`self.UT_BinaryTreeInsertData`)
  (`self.UT_BinaryTreeInsertionOrder`)
  (`self.UT_BinarySearchFunction`)
  (`self.UT_OrderSearchFunction`)
  (`self.UT_InOrderTraversal`)
  (`self.UT_ReverseOrderTraversal`)
  (`self.UT_LinklistInsertStart`)
  (`self.UT_LinkListAddNode`)
  (`self.UT_LinkListDelAtPos`)
  (`self.UT_GetPos`)
  (`self.UT_StackPush`)
  (`self.UT_StackPop`)
  (`self.UT_StackIsEmpty`)
  (`self.UT_StackPeek`))

(event `self.ReceiveTick`
  (params (DeltaSeconds :type "Float (single-precision)")))

(fn `UserConstructionScript`)